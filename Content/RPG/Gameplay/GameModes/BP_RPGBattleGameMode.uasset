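; Game mode Blueprint for RPG battles, exposing events to start and run a battle.
; Starting a battle splits the given characters into allies and enemies relative to the controlled pawn, then passes them to StartBattle; running forwards the initiating team to RunBattle.
; Turn-end and battle-finished events only print debug strings.
; The battle game mode getter returns self, while the normal-world getter returns nothing.
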(event Custom|StartRPGBattle
  (params (Characters :type Array%20of%20RPG%20Character%20Base%20Object%20References) (PlayerController :type RPG%20Player%20Controller%20Object%20Reference))
  (bind (_out_enemies _out_allies) (CallFunction|GetAlliesandEnemiesfromArray (.AsRPGCharacter%20Base (Utilities|Casting|CastToRPGCharacterBase (Pawn|GetControlledPawn PlayerController))) Characters))
  (Class|RPGBattleGameMode|StartBattle _out_enemies _out_allies PlayerController))

(event Custom|RunRPGBattle
  (params (TeamToInitiate :type ERPGTeam%20Enum :default "Neutral"))
  (Class|RPGBattleGameMode|RunBattle TeamToInitiate))

(event EventOnPlayerTurnEnded
  (Development|PrintString "Player Turn Ended"))

(event EventOnTeamTurnEnded
  (params (LastTeaminBattle :type ERPGTeam%20Enum :default "Neutral"))
  (Development|PrintString (Utilities|String|EnumtoString LastTeaminBattle)))

(event EventOnBattleFinished
  (Development|PrintString "Battle Finished"))

(fn ConstructionScript)

(fn GetBattleGameMode
  (return self))

(fn GetNormalWorldGameMode
  (return 0))