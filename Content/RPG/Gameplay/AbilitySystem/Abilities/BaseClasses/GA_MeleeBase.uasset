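; Base melee Gameplay Ability for RPG heroes that plays a stack-indexed montage combo.
; Each blend-out commits and increments a stack after a net sync, then a new press plays the next montage.
; Reaching max stacks or letting the post-release recast window expire triggers cooldown.
; Montage events build damage-modified effect containers, applied through an instant team-filtered target actor placed ahead of the right-hand weapon socket.
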(event Ability|EventActivateAbility
  (bind _asbp_rpghero_character (Utilities|Casting|CastToBP_RPGHeroCharacter (Ability|GetAvatarActorfromActorInfo)))
  (bind _output_get (Variables|Default|SetPlayer _asbp_rpghero_character))
  (Utilities|IsValid _output_get
    (:Is%20Valid
      (Ability|CommitAbility)
      (if (not (Variables|Default|GetbHasEnded)) :!label _label
        (bind (_asynctaskproxy _eventtag _eventdata) (|PlayMontageandWaitforEvent "None" (Utilities|Array|Get(acopy) (Variables|Default|GetCharacterMontagesToPlay) (Variables|Default|GetAbilityStacks)) "(GameplayTags=((TagName=\"Event.Ability.MainAbility\")))" 1.0 false "None" 1.0)
          (:then
            (bind _waitdelaytask (Variables|Default|GetWaitDelayTask)
              (:then
                (GameplayTasks|EndTask _waitdelaytask))
              (:else)))
          (:OnBlendOut
            (bind _return (CallFunction|CommitAbilityStacks))
            (if _return
              (Ability|Tasks|WaitNetSync "BothWait"
                (:OnSync
                  (Math|Integer|IncrementInt (Variables|Default|GetAbilityStacks)
                    (:%20%20
                      (Ability|Tasks|WaitInputRelease true
                        (:then
                          (Ability|Tasks|WaitInputPress false
                            (:OnPress
                              (if (CallFunction|IsMaxStacks)
                                (Ability|EndAbility :!label _label_2)
                                (else
                                  (goto _label))))))
                        (:OnRelease
                          (if (CallFunction|IsMaxStacks)
                            (CallFunction|ApplyCoolDown :!label _label_3)
                            (Utilities|FlowControl|Delay 0.2)
                            (Ability|EndAbility)
                            (else
                              (bind _asynctaskproxy_2 (Ability|Tasks|WaitDelay (Variables|Default|GetRecastTime))
                                (:then
                                  (Variables|Default|SetWaitDelayTask _asynctaskproxy_2))
                                (:OnFinish
                                  (goto _label_3)))))))))))
              (else
                (Class|RPGGameplayAbility|ResetAbilityStacks :!label _label_4)
                (goto _label_2))))
          (:OnInterrupted
            (goto _label_4))
          (:OnCancelled
            (goto _label_4))
          (:EventReceived
            (bind _returnvalue (Class|RPGGameplayAbility|MakeEffectContainerSpec _eventtag _eventdata -1))
            (bind _containerspec (Class|RPGGameplayAbility|ApplyDamageModifiers _returnvalue))
            (Variables|Default|SetContainerEffectSpec _containerspec)
            (bind _data (|WaitTargetData :ConfirmationType "Instant" :Class "/Script/RPG.RPGAbilityTargetActor" :RPGFilter (Class|RPGBlueprintFunctionLibrary|MakeRPGGameplayTargetDataFilterHandle (Utilities|Struct|MakeRPGGameplayTargetDataFilter (Class|RPGHeroCharacter|GetTeam (Variables|Default|GetPlayer)) "TDFS_NoSelf" 0 false) (Variables|Default|GetPlayer)) :Radius 1e+02 :ObjectTypes (Utilities|Array|MakeArray "ObjectTypeQuery3") :IgnoreActors (Utilities|Array|MakeArray 0) :DrawDebug "ForDuration" :StartLocation (Utilities|Struct|MakeGameplayAbilityTargetingLocationInfo "LiteralTransform" (Math|Transform|MakeTransform (Math|Vector|MakeVector (+ (.x (* (Math|Vector|Normalize (Math|Vector|GetForwardVector (Variables|/Script/Engine.Character|GetCapsuleComponent (Variables|Default|GetPlayer)))) (Math|Float|MakeLiteralFloat 6e+01))) (.X (Math|Vector|BreakVector (Transformation|GetSocketLocation (Variables|/Script/Engine.Character|GetMesh (Variables|Default|GetPlayer)) "hand_rWeapon")))) (+ (.y (* (Math|Vector|Normalize (Math|Vector|GetForwardVector (Variables|/Script/Engine.Character|GetCapsuleComponent (Variables|Default|GetPlayer)))) (Math|Float|MakeLiteralFloat 6e+01))) (.Y (Math|Vector|BreakVector (Transformation|GetSocketLocation (Variables|/Script/Engine.Character|GetMesh (Variables|Default|GetPlayer)) "hand_rWeapon")))) (.Z (Math|Vector|BreakVector (Transformation|GetSocketLocation (Variables|/Script/Engine.Character|GetMesh (Variables|Default|GetPlayer)) "hand_rWeapon")))) "0, 0, 0" "1,1,1") (Variables|Default|GetPlayer) 0 0 "hand_rWeapon") :ReticleClass 0)
              (:then
                (Class|RPGBlueprintFunctionLibrary|ApplyEffectContainerSpectoTargetsfromTargetData (Variables|Default|GetContainerEffectSpec) _data)))))))))

(event EventApplyCoolDown
  (Variables|Default|SetbHasEnded true)
  (Class|RPGGameplayAbility|ResetAbilityStacks)
  (Class|RPGGameplayAbility|ApplyRPGCoolDown))