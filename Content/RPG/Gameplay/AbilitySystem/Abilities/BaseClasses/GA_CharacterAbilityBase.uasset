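; Base Gameplay Ability class for RPG characters, providing shared helpers for stack checks and gameplay effect creation.
; MakeEffectSpec builds an outgoing effect spec from the character's Ability System Component, scaled to the character's level.
; IsMaxStacks tests for the stack cap, while CommitAbilityStacks only checks that stacks are within it, without changing the count.
; ApplyCoolDown, activation and end events are empty.
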(event Ability|EventActivateAbility)

(event Ability|EventOnEndAbility
  (params (bWasCancelled :type Boolean)))

(fn ApplyCoolDown)

(fn IsMaxStacks
  (return (== (Variables|Default|GetAbilityStacks) (Variables|Default|GetAbilityMaxStacks))))

(fn MakeEffectSpec
  (params (Character :type RPG%20Character%20Base%20Object%20Reference) (Gameplayeffect :type Gameplay%20Effect%20Class%20Reference))
  (bind _returnvalue (Ability|GetAbilitySystemComponent Character))
  (return (GameplayEffects|MakeOutgoingSpec _returnvalue Gameplayeffect (Class|RPGCharacterBase|GetCharacterLevel Character) (GameplayEffects|MakeEffectContext _returnvalue))))

(fn CommitAbilityStacks
  (return (<= (Variables|Default|GetAbilityStacks) (Variables|Default|GetAbilityMaxStacks))))