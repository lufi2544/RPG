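; Base hero melee attack ability that plays the montage indexed by the current ability stack count.
; On the MainAbility montage event it builds a damage-modified effect container and runs instant, team-filtered target data around a point offset forward from the right-hand weapon socket.
; Valid targets receive the effects.
; Montage completion resets the stacks, applies the RPG cooldown and ends the ability.
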(event Ability|EventActivateAbility
  (bind _asbp_rpghero_character (Utilities|Casting|CastToBP_RPGHeroCharacter (Ability|GetAvatarActorfromActorInfo)))
  (bind _output_get (Variables|Default|SetRPG_Player _asbp_rpghero_character))
  (Utilities|IsValid _output_get
    (:Is%20Valid
      (Ability|CommitAbility)
      (bind (_asynctaskproxy _eventtag _eventdata) (|PlayMontageandWaitforEvent "None" (Utilities|Array|Get(acopy) (Variables|Default|GetCharacterMontagesToPlay) (Variables|Default|GetAbilityStacks)) "(GameplayTags=((TagName=\"Event.Ability.MainAbility\")))" 1.0 false "None" 1.0)
        (:OnCompleted
          (Class|RPGGameplayAbility|ApplyCooldown)
          (Ability|EndAbility))
        (:EventReceived
          (bind _returnvalue (Class|RPGGameplayAbility|MakeEffectContainerSpec _eventtag _eventdata -1))
          (bind _containerspec (Class|RPGGameplayAbility|ApplyDamageModifiers _returnvalue))
          (Variables|Default|SetMainEffectContainerSpec _containerspec)
          (bind _data (|WaitTargetData :ConfirmationType "Instant" :Class "/Script/RPG.RPGAbilityTargetActor" :RPGFilter (Class|RPGBlueprintFunctionLibrary|MakeRPGGameplayTargetDataFilterHandle (Utilities|Struct|MakeRPGGameplayTargetDataFilter (Class|RPGHeroCharacter|GetTeam (.AsBP%20RPGHero%20Character (Utilities|Casting|CastToBP_RPGHeroCharacter (Variables|Default|GetRPG_Player)))) "TDFS_NoSelf" 0 false) (Variables|Default|GetRPG_Player)) :Radius 1e+02 :ObjectTypes (Utilities|Array|MakeArray "ObjectTypeQuery3") :StartLocation (Utilities|Struct|MakeGameplayAbilityTargetingLocationInfo "LiteralTransform" (Math|Transform|MakeTransform (Math|Vector|MakeVector (+ (.x (* (Math|Vector|Normalize (Math|Vector|GetForwardVector (Variables|/Script/Engine.Character|GetCapsuleComponent (Variables|Default|GetRPG_Player)))) (Math|Float|MakeLiteralFloat 6e+01))) (.X (Math|Vector|BreakVector (Transformation|GetSocketLocation (Variables|/Script/Engine.Character|GetMesh (Variables|Default|GetRPG_Player)) "hand_rWeapon")))) (+ (.y (* (Math|Vector|Normalize (Math|Vector|GetForwardVector (Variables|/Script/Engine.Character|GetCapsuleComponent (Variables|Default|GetRPG_Player)))) (Math|Float|MakeLiteralFloat 6e+01))) (.Y (Math|Vector|BreakVector (Transformation|GetSocketLocation (Variables|/Script/Engine.Character|GetMesh (Variables|Default|GetRPG_Player)) "hand_rWeapon")))) (.Z (Math|Vector|BreakVector (Transformation|GetSocketLocation (Variables|/Script/Engine.Character|GetMesh (Variables|Default|GetRPG_Player)) "hand_rWeapon")))) "0, 0, 0" "1,1,1") (Variables|Default|GetRPG_Player) 0 0 "hand_rWeapon") :ReticleClass "/Game/RPGReticle.RPGReticle_C")
            (:ValidData
              (Class|RPGBlueprintFunctionLibrary|ApplyEffectContainerSpectoTargetsfromTargetData (Variables|Default|GetMainEffectContainerSpec) _data))))))))

(event EventApplyCooldown
  (Class|RPGGameplayAbility|ResetAbilityStacks)
  (Class|RPGGameplayAbility|ApplyRPGCoolDown))