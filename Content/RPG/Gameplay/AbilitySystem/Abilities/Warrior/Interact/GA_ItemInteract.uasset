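; Gameplay ability that lets the hero character interact with an equipable item in front of them.
; The server sphere-traces forward, ignoring equipped items, and ends early without an unequipped item; non-server instances skip straight to the montage.
; The montage's interact event sends the item an interact message, then the WeaponStateHandle macro reads inventory weapon state to apply the matching primary-weapon-equipped GameplayEffect.
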(event Ability|EventActivateAbility
  (bind _asbp_rpghero_character (Utilities|Casting|CastToBP_RPGHeroCharacter (Ability|GetAvatarActorfromActorInfo)))
  (Utilities|IsValid _asbp_rpghero_character
    (:Is%20Valid
      (Variables|Default|SetPlayer _asbp_rpghero_character)
      (bind _asbp_rpgplayer_state (Utilities|Casting|CastToBP_RPGPlayerState (Variables|/Script/Engine.Pawn|GetPlayerState (Variables|Default|GetPlayer))))
      (if (Utilities|IsServer)
        (bind (_outhit _returnvalue) (Collision|SphereTraceByChannel (Math|Vector|MakeVector (.X (Math|Vector|BreakVector (Transformation|GetActorLocation (Variables|Default|GetPlayer)))) (.Y (Math|Vector|BreakVector (Transformation|GetActorLocation (Variables|Default|GetPlayer)))) (- (.Z (Math|Vector|BreakVector (Transformation|GetActorLocation (Variables|Default|GetPlayer)))) 15.0)) (+ (Math|Vector|MakeVector (.X (Math|Vector|BreakVector (Transformation|GetActorLocation (Variables|Default|GetPlayer)))) (.Y (Math|Vector|BreakVector (Transformation|GetActorLocation (Variables|Default|GetPlayer)))) (- (.Z (Math|Vector|BreakVector (Transformation|GetActorLocation (Variables|Default|GetPlayer)))) 15.0)) (* (Math|Vector|GetForwardVector (Variables|/Script/Engine.Character|GetCapsuleComponent (Variables|Default|GetPlayer))) 5e+02)) 7e+01 "TraceTypeQuery1" false (Class|RPGPlayerInventoryComponent|GetEquippedItems (Variables|/Script/RPG.RPGPlayerState|GetInventoryComponent _asbp_rpgplayer_state)) "None"))
        (if _returnvalue
          ;[1 1 0] Add the Animation Montage Setter, it could be a rope, or maybe a ladder
          (bind _asrpgequipable_item (Utilities|Casting|CastToRPGEquipableItem (.HitActor (Collision|BreakHitResult _outhit)))
            (:then
              (if (Variables|/Script/RPG.RPGEquipableItem|GetbIsEquipped _asrpgequipable_item)
                (Ability|EndAbility :!label _label)
                (else
                  (|PlayMontageandWaitforEvent "None" (Variables|Default|GetInteractionMontage) "(GameplayTags=((TagName=\"Event.Montage.Ability.Interact\")))" 1.0 true "None" 1.0 :!label _label_2
                    (:OnCompleted
                      (goto _label))
                    (:OnInterrupted
                      (goto _label))
                    (:OnCancelled
                      (goto _label))
                    (:EventReceived
                      (Class|BPItemInterface|InterctwithItem(Message) (.AsRPGEquipable%20Item (Utilities|Casting|CastToRPGEquipableItem (.HitActor (Collision|BreakHitResult _outhit)))) (Variables|Default|GetPlayer) (.AsRPGEquipable%20Item (Utilities|Casting|CastToRPGEquipableItem (.HitActor (Collision|BreakHitResult _outhit)))))
                      (Utilities|WeaponStateHandle
                        (:AllPrimaryWeaponsEquipped
                          (Ability|ApplyGameplayEffectToOwner "/Game/RPG/Gameplay/AbilitySystem/Effects/Shared/GE_Inventory_AllPrimaryWeaponsEquipped.GE_Inventory_AllPrimaryWeaponsEquipped_C"))
                        (:PrimaryWeaponEquipped
                          (Ability|ApplyGameplayEffectToOwner "/Game/RPG/Gameplay/AbilitySystem/Effects/Shared/GE_Inventory_WeaponEquipped.GE_Inventory_WeaponEquipped_C"))))))))
            (:CastFailed
              (goto _label)))
          (else
            (goto _label)))
        (else
          (goto _label_2))))))