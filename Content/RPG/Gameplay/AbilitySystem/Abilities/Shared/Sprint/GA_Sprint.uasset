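; Gameplay ability that makes the RPG hero character sprint while the ability input is held.
; On activation it applies the GE_SprintEffect gameplay effect, stores its handle and calls StartSprinting on the RPG character movement component.
; A WaitInputRelease task ends the ability when the input is released.
; On end it removes the stored effect and calls StopSprinting on the movement component.
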(event Ability|EventActivateAbility
  (bind _asbp_rpghero_character (Utilities|Casting|CastToBP_RPGHeroCharacter (Ability|GetAvatarActorfromActorInfo)))
  (Variables|Default|SetPlayer _asbp_rpghero_character)
  (bind _returnvalue (Ability|ApplyGameplayEffectToOwner "/Game/RPG/Gameplay/AbilitySystem/Abilities/Shared/Sprint/GE_SprintEffect.GE_SprintEffect_C"))
  (Variables|Default|SetSprintActiveHandle _returnvalue)
  (bind _asrpgcharacter_movement_component (Utilities|Casting|CastToRPGCharacterMovementComponent (.MovementComponent (Utilities|Struct|BreakGameplayAbilityActorInfo (Ability|GetActorInfo)))))
  (Class|RPGCharacterMovementComponent|StartSprinting _asrpgcharacter_movement_component)
  ;[1 1 1] We add a wait input realese for the ability, so we can run the StopAbility mehtod on the Movement Component
  (Ability|Tasks|WaitInputRelease true
    (:OnRelease
      (Ability|EndAbility))))

(event Ability|EventOnEndAbility
  (params (bWasCancelled :type Boolean))
  (Ability|RemoveGameplayEffectFromOwnerWithHandle (Variables|Default|GetSprintActiveHandle))
  (bind _asrpgcharacter_movement_component (Utilities|Casting|CastToRPGCharacterMovementComponent (.MovementComponent (Utilities|Struct|BreakGameplayAbilityActorInfo (Ability|GetActorInfo)))))
  (Class|RPGCharacterMovementComponent|StopSprinting _asrpgcharacter_movement_component))