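; Blueprint function library for the RPG, providing a debug print helper and a function that sorts characters into allies and enemies.
; RPGPrintString prints display names for an array's elements, or for a single valid actor when the array is empty.
; GetAlliesAndEnemiesFromArray adds the player as an ally, then uses IsPlayerAlly to cast each other player into unique hero ally or RPGEnemy arrays.
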(fn RPGPrintString
  (params (Array :type Array%20of%20Actor%20Object%20References) (Actor :type Actor%20Object%20Reference))
  (if (> (Utilities|Array|Length Array) 0)
    (for _array_element Array
      (Development|PrintString _array_element (Utilities|GetDisplayName _array_element)))
    (else
      (Utilities|IsValid Actor
        (:Is%20Valid
          (Development|PrintString Actor (Utilities|GetDisplayName Actor)))))))

(fn GetAlliesandEnemiesfromArray
  (params (Player :type RPG%20Character%20Base%20Object%20Reference) (OtherPlayers :type Array%20of%20RPG%20Character%20Base%20Object%20References))
  (Utilities|Array|AddUnique (LocalVariables|GetAllies) (.AsBP%20RPGHero%20Character (Utilities|Casting|CastToBP_RPGHeroCharacter Player)))
  (for _array_element OtherPlayers
    (if (Class|RPGBlueprintFunctionLibrary|IsPlayerAlly Player _array_element)
      (Utilities|Array|AddUnique (LocalVariables|GetAllies) (.AsBP%20RPGHero%20Character (Utilities|Casting|CastToBP_RPGHeroCharacter _array_element)))
      (else
        (Utilities|Array|AddUnique (LocalVariables|GetEnemies) (.AsRPGEnemy (Utilities|Casting|CastToRPGEnemy _array_element))))))
  (return (LocalVariables|GetEnemies) (LocalVariables|GetAllies)))