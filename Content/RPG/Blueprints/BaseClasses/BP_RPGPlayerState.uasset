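; BP_RPGPlayerState is the RPG player state, holding the player's inventory and current animation mode.
; Item data is appended to an array while a counter tracks usage against a capacity taken from the bag.
; The capacity check is a separate function, so adding an item does not enforce the limit itself.
; Animation mode is looked up by weapon type in a map and changes only when an entry exists.
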(event EventBeginPlay)

(event EventTick
  (params (DeltaSeconds :type Float%20%28single-precision%29)))

(fn ConstructionScript)

(fn AddItemDatatoInventory
  (params (InItemData :type RPG%20Item%20Data%20Structure))
  (Utilities|Array|Add (Variables|RPG|RPGPlayerState|Item|GetInventoryItemDataArray) InItemData)
  (Math|Integer|IncrementInt (Variables|RPG|RPGPlayerState|Item|GetPlayerCurrentCapacity)))

(fn SetAnimationState
  (params (InWeaponType :type ERPGWeaponType%20Enum :default "None"))
  (bind _characteranimationmap (Variables|RPG|RPGPlayerState|Item|GetCharacterAnimationMap))
  (bind (_value _returnvalue) (Utilities|Map|Find _characteranimationmap InWeaponType))
  (if _returnvalue
    (Variables|RPG|RPGPlayerState|Item|SetAnimationMode _value)))

(fn SetInventoryCapacity
  (params (Bag :type RPG%20Bag%20Object%20Reference))
  (Variables|RPG|RPGPlayerState|Item|SetPlayerInventoryCapacity (Variables|/Script/RPG.RPGBag|GetBagCapacity Bag)))

(fn CheckInventoryCapacity
  (if (< (Variables|RPG|RPGPlayerState|Item|GetPlayerCurrentCapacity) (Variables|RPG|RPGPlayerState|Item|GetPlayerInventoryCapacity))
    (return true)
    (else
      (return false))))