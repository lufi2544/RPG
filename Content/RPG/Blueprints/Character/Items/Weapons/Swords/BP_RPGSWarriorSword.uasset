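; Warrior sword item Blueprint that handles a player picking up or equipping the sword.
; InterctWithItem switches on item type and, for weapons, asks the RPG player state to equip the item on the right-hand weapon socket.
; If equipping fails, it adds the item data to the player state's inventory, destroys the actor and returns false.
; The event graph holds only disabled default events.
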(event EventBeginPlay
  (|CallParentFunction) ; This node is disabled and will not be called.\nDrag off pins to build functionality.
)

(event Collision|EventActorBeginOverlap
  (params (OtherActor :type Actor%20Object%20Reference))
  (|CallParentFunction OtherActor) ; This node is disabled and will not be called.\nDrag off pins to build functionality.
)

(event EventTick
  (params (DeltaSeconds :type Float%20%28single-precision%29))
  (|CallParentFunction DeltaSeconds) ; This node is disabled and will not be called.\nDrag off pins to build functionality.
)

(fn ConstructionScript
  (|CallParentFunction))

(fn InterctwithItem
  (params (Player :type RPG%20Character%20Base%20Object%20Reference) (Item :type RPG%20Equipable%20Item%20Object%20Reference))
  (bind _returnvalue (Class|RPGEquipableItem|GetItemData Item))
  (bind _playerstate (Variables|/Script/Engine.Pawn|GetPlayerState Player))
  (bind _asrpgplayer_state (Utilities|Casting|CastToRPGPlayerState _playerstate))
  (switch Utilities|FlowControl|Switch|SwitchonERPGItemType (Utilities|Struct|BreakRPGItemData _returnvalue)
    (:Weapon
      (bind _returnvalue_2 (Class|RPGPlayerState|EquipItem _asrpgplayer_state Item Player "hand_rWeapon"))
      (if _returnvalue_2
        _
        (else
          (Default|AddItemDatatoInventory (.AsBP%20RPGPlayer%20State (Utilities|Casting|CastToBP_RPGPlayerState _asrpgplayer_state)) _returnvalue)
          (Actor|DestroyActor Item)))
      (return _returnvalue_2))))